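; Drift_Base is a hovering car base that floats over tagged surfaces and drives forward while W is held.
; Each tick it traces between two DriveHeight spline points and matches the hit component's tags against EDriverCollision names.
; On a match it disables gravity, zeroes velocity once, interpolates toward a height above the impact and applies gated forward impulses; otherwise gravity returns.
; RightUpOnHit, which also aligns rotation to the surface, is unused.
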(event Custom|ExecuteMovement
  (Utilities|FlowControl|Sequence
    (:then_0
      ;[1 1 1] Forward
      (Utilities|FlowControl|Gate true
        (:Exit
          (Physics|AddImpulse (Variables|Default|GetCar) (* (Transformation|GetActorForwardVector) (* (Variables|Default|GetMultiplier) (Variables|Default|GetForwardSpeed))) "None" false))))))

(event EventTick
  (params (DeltaSeconds :type Float%20%28single-precision%29))
  (bind _car (Variables|Default|GetCar))
  (bind (_hashit _hitresult) (CallFunction|RegisterHit))
  (bind (_canfloat _hit _edrivercollision) (CallFunction|HandleHit _hashit _hitresult))
  (if _canfloat
    (Physics|SetEnableGravity _car false)
    (if (Variables|Default|GetCanNullifyPhysics)
      (Class|PrimitiveComponent|SetAllPhysicsLinearVelocity (Variables|Default|GetCar) "0, 0, 0" false)
      (Variables|Default|SetCanNullifyPhysics false))
    (CallFunction|RightUp _hit (Transformation|GetActorTransform) _edrivercollision DeltaSeconds)
    (CallFunction|ExecuteMovement)
    (else
      (Physics|SetEnableGravity _car true)
      (if (not (Variables|Default|GetCanNullifyPhysics))
        (Variables|Default|SetCanNullifyPhysics true)))))

(event Input|KeyboardEvents|W
  (params (Key :type Key%20Structure :default "AnyKey"))
  ;[1 1 1] Forward
  (:Pressed
    (Utilities|FlowControl|Gate true) ; enters at Open
  )
  (:Released
    (Utilities|FlowControl|Gate true) ; enters at Close
  ))

(fn ConstructionScript)

(fn RegisterHit
  (bind (_outhit _returnvalue) (Collision|LineTraceForObjects (Spline|GetLocationatSplinePoint (Variables|Default|GetDriveHeight) 0 "World") (Spline|GetLocationatSplinePoint (Variables|Default|GetDriveHeight) 1 "World") (LocalVariables|GetEObjectType) false 0 "None"))
  (return _returnvalue _outhit))

(fn HandleHit
  (params (HasResult :type Boolean) (HitResult :type Hit%20Result%20Structure))
  (if HasResult
    (bind _array_element (Utilities|Array|ForEachLoopwithBreak (Variables|/Script/Engine.ActorComponent|GetComponentTags (.HitComponent (Collision|BreakHitResult HitResult))))
      (:LoopBody
        (bind _enumvalue (|ForEachEDriverCollision)
          (:LoopBody
            (if (Utilities|Enum|Equal(Enum) (Utilities|String|EnumtoString _enumvalue) (Class|KismetStringLibrary|ToUpper (Utilities|String|ToString(Name) _array_element)))
              (return true HitResult _enumvalue)
              (else
                _)))))
      (:Completed
        _)))
  (return false "" "NewEnumerator0"))

(fn RightUponHit
  (params (HitResult :type Hit%20Result%20Structure) (ThisTransform :type Transform) (EDriverCollision :type EDriverCollision%20Enum) (TimeSeconds :type Float%20%28single-precision%29))
  (bind _returnvalue (Transformation|GetActorForwardVector))
  (bind (_bblockinghit _binitialoverlap _time _location _impactpoint _normal _impactnormal) (Collision|BreakHitResult HitResult))
  (LocalVariables|SetLocalTimeSeconds TimeSeconds)
  (Utilities|FlowControl|Sequence
    (:then_0
      ;[1 1 1] Set object to hit location and shift up from location
      (bind _output_get (LocalVariables|Setspot _impactpoint))
      (bind _output_get_2 (LocalVariables|Settarget ThisTransform))
      (bind _output_get_3 (LocalVariables|Settarget (Math|Transform|MakeTransform _output_get (.Rotation (Math|Transform|BreakTransform _output_get_2)) (.Scale (Math|Transform|BreakTransform _output_get_2)))))
      (LocalVariables|Settarget (Math|Transform|MakeTransform (+ (.Location (Math|Transform|BreakTransform _output_get_3)) (* (Math|Vector|GetUpVector (Math|Conversions|RotationFromXVector (.Location (Math|Transform|BreakTransform _output_get_3)))) (Variables|Default|GetBaseHeight))) (.Rotation (Math|Transform|BreakTransform _output_get_3)) (.Scale (Math|Transform|BreakTransform _output_get_3))))
      (Transformation|SetActorLocation (Math|Interpolation|VInterpTo (.Location (Math|Transform|BreakTransform ThisTransform)) (+ (.Location (Math|Transform|BreakTransform _output_get_3)) (* (Math|Vector|GetUpVector (Math|Conversions|RotationFromXVector (.Location (Math|Transform|BreakTransform _output_get_3)))) (Variables|Default|GetBaseHeight))) (LocalVariables|GetLocalTimeSeconds) 1e+01) true false))
    (:then_1
      ;[1 1 1] Rotate player
      (LocalVariables|SetnewForward (- _returnvalue (* _impactnormal (Math|Vector|DotProduct _returnvalue _impactnormal))))
      (LocalVariables|SetnewRotation (Math|Rotator|GetRotationXVector (Math|Rotator|MakeRotfromXZ (LocalVariables|GetnewForward) _impactnormal)))
      (Transformation|SetActorRotation (Math|Rotator|Lerp(Rotator) (Transformation|GetActorRotation) (Math|Conversions|RotationFromXVector (LocalVariables|GetnewRotation)) (* (LocalVariables|GetLocalTimeSeconds) 5.0))))))

(fn RightUp
  (params (HitResult :type Hit%20Result%20Structure) (ThisTransform :type Transform) (EDriverCollision :type EDriverCollision%20Enum) (TimeSeconds :type Float%20%28single-precision%29))
  (LocalVariables|SetLocalTimeSeconds TimeSeconds)
  (Utilities|FlowControl|Sequence
    (:then_0
      ;[1 1 1] Set object to hit location and shift up from location
      (bind _output_get (LocalVariables|Setspot (.ImpactPoint (Collision|BreakHitResult HitResult))))
      (bind _output_get_2 (LocalVariables|Settarget ThisTransform))
      (bind _output_get_3 (LocalVariables|Settarget (Math|Transform|MakeTransform _output_get (.Rotation (Math|Transform|BreakTransform _output_get_2)) (.Scale (Math|Transform|BreakTransform _output_get_2)))))
      (LocalVariables|Settarget (Math|Transform|MakeTransform (+ (.Location (Math|Transform|BreakTransform _output_get_3)) (* (Math|Vector|GetUpVector (Math|Conversions|RotationFromXVector (.Location (Math|Transform|BreakTransform _output_get_3)))) (Variables|Default|GetBaseHeight))) (.Rotation (Math|Transform|BreakTransform _output_get_3)) (.Scale (Math|Transform|BreakTransform _output_get_3))))
      (Transformation|SetActorLocation (Math|Interpolation|VInterpTo (.Location (Math|Transform|BreakTransform ThisTransform)) (+ (.Location (Math|Transform|BreakTransform _output_get_3)) (* (Math|Vector|GetUpVector (Math|Conversions|RotationFromXVector (.Location (Math|Transform|BreakTransform _output_get_3)))) (Variables|Default|GetBaseHeight))) (LocalVariables|GetLocalTimeSeconds) 1e+01) true false))))